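; BP_MoveWall is a sliding wall that acts as a keyed door to a secret room.
; On box overlap, it asks actors implementing BPI_Char whether they hold the key for its RoomId, then plays the DoorOpen timeline to slide the mesh along relative X.
; Without the key, it posts a Chinese "can't open" message through the game mode.
; When such an actor leaves the box, an open wall reverses the timeline to close.
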(event `self.Box.OnComponentBeginOverlap`
  (params (OtherActor :type "Actor Object Reference") (OtherComp :type "PrimitiveComponent Object Reference") (OtherBodyIndex :type Integer) (bFromSweep :type Boolean) (SweepResult :type "HitResult Structure (by ref)"))
  (bind _staticmesh (`self.StaticMesh`))
  (bind (_relativelocation_x _relativelocation_y _relativelocation_z) (`KismetMathLibrary.BreakVector` (`SceneComponent.RelativeLocation` _staticmesh)))
  (if (`KismetSystemLibrary.DoesImplementInterface` OtherActor "/Game/FirstPersonBP/Interfaces/BPI_Char.BPI_Char_C")
    (bind _bhave (message `/Game/FirstPersonBP/Interfaces/BPI_Char.HaveKey` OtherActor (`self.RoomId`)))
    (if _bhave
      (if (not (`self.bOpen`))
        (set `self.bOpen` true)
        (bind (_direction _openoffset) (`Timeline|DoorOpen` :`NewTime` 0.0 :!label _label)
          (:`Update`
            (`SceneComponent.K2_SetRelativeLocation` _staticmesh (`KismetMathLibrary.MakeVector` _openoffset _relativelocation_y _relativelocation_z) false false))))
      (else
        (message `/Game/FirstPersonBP/Interfaces/BPI_GameMode.AddMsg` (`GameplayStatics.GetGameMode`) (make `/Game/Message/Msg` "打不开，看来我还没有这个密室的钥匙"))))))

(event `self.Box.OnComponentEndOverlap`
  (params (OtherActor :type "Actor Object Reference") (OtherComp :type "PrimitiveComponent Object Reference") (OtherBodyIndex :type Integer))
  (if (`KismetSystemLibrary.DoesImplementInterface` OtherActor "/Game/FirstPersonBP/Interfaces/BPI_Char.BPI_Char_C")
    (if (`self.bOpen`)
      (set `self.bOpen` false)
      (goto _label :!via `Reverse`))))

(fn `UserConstructionScript`)