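; BP_End is a level goal actor that completes the game when a character reaches it.
; Each tick it spins the Core component around yaw at RotateSpeed and turns its TextRender toward the player on pitch and yaw, keeping roll unchanged.
; When an actor implementing BPI_Char overlaps the Trigger, it calls GameCompleteMessage on the game mode.
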(event `self.ReceiveTick`
  (params (DeltaSeconds :type "Float (single-precision)"))
  ;[1 1 1] Auto Rotate
  (`SceneComponent.K2_AddLocalRotation` (`self.Core`) (`KismetMathLibrary.MakeRotator` 0.0 0.0 (* (`self.RotateSpeed`) DeltaSeconds)) false false)
  ;[1 1 1] 设置文字角度
  (`SceneComponent.K2_SetWorldRotation` (`self.TextRender`) (`KismetMathLibrary.MakeRotator` (.roll (`SceneComponent.K2_GetComponentRotation` (`self.TextRender`))) (.pitch (`KismetMathLibrary.FindLookAtRotation` (`SceneComponent.K2_GetComponentLocation` (`self.TextRender`)) (`self.K2_GetActorLocation` (`GameplayStatics.GetPlayerCharacter` 0)))) (.yaw (`KismetMathLibrary.FindLookAtRotation` (`SceneComponent.K2_GetComponentLocation` (`self.TextRender`)) (`self.K2_GetActorLocation` (`GameplayStatics.GetPlayerCharacter` 0))))) false false))

(event `self.Trigger.OnComponentBeginOverlap`
  (params (OtherActor :type "Actor Object Reference") (OtherComp :type "PrimitiveComponent Object Reference") (OtherBodyIndex :type Integer) (bFromSweep :type Boolean) (SweepResult :type "HitResult Structure (by ref)"))
  ;[1 1 1] 玩家进入，游戏任务完成
  (if (`KismetSystemLibrary.DoesImplementInterface` OtherActor "/Game/FirstPersonBP/Interfaces/BPI_Char.BPI_Char_C")
    (message `/Game/FirstPersonBP/Interfaces/BPI_GameMode.GameComplete` (`GameplayStatics.GetGameMode`))))

(fn `UserConstructionScript`)