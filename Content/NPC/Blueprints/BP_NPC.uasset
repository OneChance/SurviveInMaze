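; NPC Blueprint that handles health, threat tracking and death loot for an enemy that targets the player.
; Health reaching zero spawns an explosion and the Pickups list, which SetPickupsByLevel fills with level-scaled ammo or battery.
; Tick follows the last attacker, otherwise the Blackboard target, clearing the Blackboard target on its death or after accumulated time without line of sight.
; NotiAttackAnimCancel is an empty hook called on target death; the separate patrol-threat timer is unconnected.
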(event `/Game/NPC/Interfaces/BPI_NPC.HealthChange`
  (params (ChangeValue :type Integer))
  ;[1 1 1] 生命值变化
  (bind _output_get (set `self.CurrentHealth` (`KismetMathLibrary.Max` (`KismetMathLibrary.Min` (+ (`self.CurrentHealth`) ChangeValue) (`self.MaxHealth`)))))
  (if (== _output_get 0)
    (`GameplayStatics.SpawnEmitterAtLocation` "/Game/Effects/ParticleSystems/P_Explosion_Bomb.P_Explosion_Bomb" (`self.K2_GetActorLocation` self))
    (for _array_element (`self.Pickups`)
      (bind _returnvalue (`|SpawnActorFromClass` (`.PClass_11_59E997408A40EC4CE0C781B1A464EDFB` (break `/Game/Pickups/PickupInfo` _array_element)) (`KismetMathLibrary.MakeTransform` (+ (`self.K2_GetActorLocation` self) (0.0 0.0 -50.0))) "Undefined" "OverrideRootScale"))
      (set `/Game/Pickups/Blueprints/Pickups.PNum` (`.PNum_8_45F2414DE24530A6744ED68F984FDAF8` (break `/Game/Pickups/PickupInfo` _array_element)) _returnvalue))
    (`self.K2_DestroyActor`)))

(event `/Game/NPC/Interfaces/BPI_NPC.Attacked`
  (params (AttackedBy :type "Actor Object Reference"))
  ;[1 1 1] 当被攻击时 直接锁定目标
  (set `self.TargetWhoAttackActor` AttackedBy)
  (set `self.AttackedThreatRemoveTimer` 0.0))

(event `self.ReceiveTick`
  (params (DeltaSeconds :type "Float (single-precision)"))
  (bind _currenttarget (`self.CurrentTarget`))
  (bind _returnvalue (`BlackboardComponent.GetValueAsObject` (`AIBlueprintHelperLibrary.GetBlackboard` self) (`self.BB_Target`)))
  (if (!= (`self.TargetWhoAttackActor`) null)
    (set `self.CurrentTarget` (`self.TargetWhoAttackActor`))
    (bind _balive (`self.IsAlive` _currenttarget :!label _label)) ; 如果目标死亡，移除目标
    (if _balive
      (bind _bvisible (`self.TargetIsVisble` _currenttarget)) ; 如果目标不可见，开始计时，时间到后移除目标
      (if (not _bvisible)
        ;[1 1 1] 有攻击仇恨目标的情况
        (bind _output_get (set `self.AttackedThreatRemoveTimer` (+ DeltaSeconds (`self.AttackedThreatRemoveTimer`))))
        (if (> _output_get (`self.AttackedThreatRemoveTime`))
          ;;[1 1 1] 移除攻击仇恨目标
          (set `self.TargetWhoAttackActor` null)
          (set `self.AttackedThreatRemoveTimer` 0.0)
          ;[1 1 1] 移除目标
          (`BlackboardComponent.SetValueAsObject` (`AIBlueprintHelperLibrary.GetBlackboard` self) (`self.BB_Target`) null :!label _label_2)))
      (else
        (`self.NotiAttackAnimCancel`)
        (goto _label_2)))
    (elif (!= _returnvalue null)
      (bind _asactor (cast `Actor` _returnvalue))
      (set `self.CurrentTarget` _asactor)
      (goto _label))))

(fn `IsAlive`
  (params (Target :type "Actor Object Reference"))
  (returns (bAlive :type Boolean))
  (bind _asfirst_person_character (cast `/Game/FirstPersonBP/Blueprints/FirstPersonCharacter` Target))
  (return (> (`/Game/FirstPersonBP/Blueprints/FirstPersonCharacter.CurrentHealth` _asfirst_person_character) 0)))

(fn `NotiAttackAnimCancel`)

(fn `SetPickupsByLevel`
  (params (Level :type Integer))
  (bind _returnvalue (* (`KismetMathLibrary.RandomIntegerInRange` 1 3) Level))
  (switch `int` (`KismetMathLibrary.RandomIntegerInRange` 0 1)
    (:`0`
      (`KismetArrayLibrary.Array_Add` (`self.Pickups`) (make `/Game/Pickups/PickupInfo` "" _returnvalue "/Game/Pickups/Blueprints/Pickups_Ammo.Pickups_Ammo_C")))
    (:`1`
      (`KismetArrayLibrary.Array_Add` (`self.Pickups`) (make `/Game/Pickups/PickupInfo` "" _returnvalue "/Game/Pickups/Blueprints/Pickups_Battery.Pickups_Battery_C")))))

(fn `TargetIsVisble`
  (params (Target :type "Actor Object Reference"))
  (returns (bVisible :type Boolean))
  (bind (_outhit _returnvalue) (`KismetSystemLibrary.LineTraceSingle` (`self.K2_GetActorLocation`) (`self.K2_GetActorLocation` Target) "TraceTypeQuery1"))
  (return (not _returnvalue)))

(fn `UserConstructionScript`)