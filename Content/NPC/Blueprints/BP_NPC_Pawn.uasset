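; BP_NPC_Pawn is an NPC pawn whose billboard sprite shows which enemy class its NPCType variable selects.
; The construction script compares NPCType against five enemy Blueprints (Ganfault, Goblin, Jill, Vampire and Mortimer) in a chain of branches and sets the matching sprite.
; Any other type leaves the sprite unchanged, and the file contains no other logic.
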(fn `UserConstructionScript`
  (if (== (`self.NPCType`) "/Game/NPC/Blueprints/Enemy/BP_Enemy_Ganfault.BP_Enemy_Ganfault_C")
    (`BillboardComponent.SetSprite` (`self.Billboard`) "/Game/NPC/Blueprints/ganfault.ganfault")
    (elif (== (`self.NPCType`) "/Game/NPC/Blueprints/Enemy/BP_Enemy_Goblin.BP_Enemy_Goblin_C")
      (`BillboardComponent.SetSprite` (`self.Billboard`) "/Game/NPC/Blueprints/goblin.goblin")
      (elif (== (`self.NPCType`) "/Game/NPC/Blueprints/Enemy/BP_Enemy_Jill.BP_Enemy_Jill_C")
        (`BillboardComponent.SetSprite` (`self.Billboard`) "/Game/NPC/Blueprints/jill.jill")
        (elif (== (`self.NPCType`) "/Game/NPC/Blueprints/Enemy/BP_Enemy_Vampire.BP_Enemy_Vampire_C")
          (`BillboardComponent.SetSprite` (`self.Billboard`) "/Game/NPC/Blueprints/v.v")
          (elif (== (`self.NPCType`) "/Game/NPC/Blueprints/Enemy/BP_Enemy_Mortimer.BP_Enemy_Mortimer_C")
            (`BillboardComponent.SetSprite` (`self.Billboard`) "/Game/NPC/Blueprints/m.m")))))))