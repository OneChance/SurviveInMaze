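; BP_Enemy_vanguard is the Vanguard enemy NPC, linking attack and death events to animation and game mode.
; AttackAnim uses a cached Mixamo Vanguard AnimBP reference, cast from the mesh when needed, to enable its attack flag.
; NotiAttackAnimCancel re-casts the anim instance to clear that flag.
; Killed notifies the game mode with this enemy's NPC ID, and construction only runs the parent script.
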(event `self.AttackAnim`
  ;[1 1 1] Attack
  (if (== (`self.Anim`) null)
    (bind _asmixamo_anim_bp_vanguard (cast `/Game/MixamoAnimPack/Mixamo_Vanguard/Anims/MixamoAnimBP_Vanguard` (`SkeletalMeshComponent.GetAnimInstance` (`self.Mesh`))))
    (set `self.Anim` _asmixamo_anim_bp_vanguard))
  (if (not (`/Game/MixamoAnimPack/Mixamo_Vanguard/Anims/MixamoAnimBP_Vanguard.EnableAttack` (`self.Anim`)))
    (set `/Game/MixamoAnimPack/Mixamo_Vanguard/Anims/MixamoAnimBP_Vanguard.EnableAttack` true (`self.Anim`))))

(event `/Game/NPC/Blueprints/BP_NPC.NotiAttackAnimCancel`
  ;[1 1 1] 停止攻击
  (bind _asmixamo_anim_bp_vanguard (cast `/Game/MixamoAnimPack/Mixamo_Vanguard/Anims/MixamoAnimBP_Vanguard` (`SkeletalMeshComponent.GetAnimInstance` (`self.Mesh`))))
  (set `/Game/MixamoAnimPack/Mixamo_Vanguard/Anims/MixamoAnimBP_Vanguard.EnableAttack` false _asmixamo_anim_bp_vanguard))

(event `/Game/NPC/Blueprints/BP_NPC.Killed`
  (message `/Game/FirstPersonBP/Interfaces/BPI_GameMode.NPCKilled` (`GameplayStatics.GetGameMode`) 4))

(fn `UserConstructionScript`
  (`parent.UserConstructionScript`))