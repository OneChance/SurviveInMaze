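; Enemy AI character Blueprint that attacks the target stored in its AI controller's Blackboard.
; The attack event casts that target to the BPI_Char interface, plays an attack animation, then after a fixed delay triggers a hit effect and applies damage through HealthChange.
; An out-of-range event cancels the attack animation; the animation and effect functions are empty here, and construction flags the character as an enemy.
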(event `AttackEvent`
  (bind _asbpi_char (cast `/Game/FirstPersonBP/Interfaces/BPI_Char` (`BlackboardComponent.GetValueAsObject` (`AIBlueprintHelperLibrary.GetBlackboard` (`self.GetController`)) (`self.Target`))))
  (`self.AttackAnim`)
  (`KismetSystemLibrary.Delay` 1.5)
  (`self.AttackEffectTarget`)
  (`/Game/FirstPersonBP/Interfaces/BPI_Char.HealthChange` _asbpi_char (`self.Damage`)))

(event `AttackRangeOut`
  (`self.AttackAnimCancel`))

(fn `AttackAnim`)

(fn `AttackAnimCancel`)

(fn `AttackEffectTarget`)

(fn `UserConstructionScript`
  (set `self.bEnemy` true))