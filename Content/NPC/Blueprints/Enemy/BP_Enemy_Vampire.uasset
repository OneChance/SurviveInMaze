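; Vampire enemy NPC Blueprint that supplies its attack animation, skin flash and target effect on top of a parent enemy class.
; Construction creates a dynamic skin material and copies combat, movement, health and threat settings into variables.
; Attack events toggle EnableAttack on the vampire AnimBP, briefly pulse the skinColor parameter, and spawn a short-lived electricity emitter near the current target.
; A destroy binding from BeginPlay removes any active effect with the actor.
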(event `self.AttackAnim`
  ;[1 1 1] 攻击动画
  (if (== (`self.Anim`) null)
    (bind _asmixamo_anim_bp_vampire (cast `/Game/MixamoAnimPack/Mixamo_Vampire/Anims/MixamoAnimBP_Vampire` (`SkeletalMeshComponent.GetAnimInstance` (`self.Mesh`))))
    (set `self.Anim` _asmixamo_anim_bp_vampire))
  (if (not (`/Game/MixamoAnimPack/Mixamo_Vampire/Anims/MixamoAnimBP_Vampire.EnableAttack` (`self.Anim`)))
    (set `/Game/MixamoAnimPack/Mixamo_Vampire/Anims/MixamoAnimBP_Vampire.EnableAttack` true (`self.Anim`)))
  (`MaterialInstanceDynamic.SetScalarParameterValue` (`self.skin_MID`) "skinColor" 0.7)
  (`KismetSystemLibrary.Delay` 0.2)
  (`MaterialInstanceDynamic.SetScalarParameterValue` (`self.skin_MID`) "skinColor" 0.0))

(event `self.AttackEffectTarget`
  (bind _currenttarget (`self.CurrentTarget`))
  ;[1 1 1] 攻击特效
  (bind _returnvalue (`GameplayStatics.SpawnEmitterAtLocation` "/Game/Effects/ParticleSystems/P_electricity_DEMOFNL.P_electricity_DEMOFNL" (+ (+ (`self.K2_GetActorLocation` _currenttarget) (* (`self.GetActorUpVector` _currenttarget) -80.0)) (* (`self.GetActorForwardVector` _currenttarget) 150.0)) (struct :`Pitch` 90.0) false))
  (bind _output_get (set `self.CurrentEffect` _returnvalue))
  (`KismetSystemLibrary.Delay` 1.0)
  (`ActorComponent.K2_DestroyComponent` _output_get))

(event `self.AttackAnimCancel`
  ;[1 1 1] 取消攻击
  (bind _asmixamo_anim_bp_vampire (cast `/Game/MixamoAnimPack/Mixamo_Vampire/Anims/MixamoAnimBP_Vampire` (`SkeletalMeshComponent.GetAnimInstance` (`self.Mesh`))))
  (set `/Game/MixamoAnimPack/Mixamo_Vampire/Anims/MixamoAnimBP_Vampire.EnableAttack` false _asmixamo_anim_bp_vampire))

(event `对象销毁`
  ;[1 1 1] 绑定销毁事件，如果当前有正在播放的特效，一起销毁
  (`ActorComponent.K2_DestroyComponent` (`self.CurrentEffect`)))

(event `self.ReceiveBeginPlay`
  ;[1 1 1] 绑定销毁事件，如果当前有正在播放的特效，一起销毁
  (add `self.OnDestroyed` (delegate `对象销毁`)))

(fn `UserConstructionScript`
  (bind __maxhealth (`self._MaxHealth`))
  (`parent.UserConstructionScript`)
  (bind _returnvalue (`PrimitiveComponent.CreateDynamicMaterialInstance` (`self.Mesh`) 1 "/Game/MixamoAnimPack/Mixamo_Vampire/Materials/Vamp_Mat.Vamp_Mat"))
  (set `self.skin_MID` _returnvalue)
  (set `self.AttackRange` (`self._AttackRange`))
  (set `self.SenseRange` (`self._SenseRange`))
  (set `self.ThreatRange` (`self._ThreatRange`))
  (set `self.bCrossWall` (`self._bCrossWall`))
  (set `self.bLongDistance` (`self._bLongDistance`))
  (set `self.RunSpeed` (`self._RunSpeed`))
  (set `self.StopDistance` (`self._StopDistance`))
  (set `self.Damage` (`self._Damage`))
  (set `self.Name` (`self._Name`))
  (set `self.CurrentHealth` __maxhealth)
  (set `self.MaxHealth` __maxhealth)
  (set `self.PatrolThreatRemoveTime` (`self._PatrolThreatRemoveTime`))
  (set `self.AttackedThreatRemoveTime` (`self._AttackedThreatRemove`)))