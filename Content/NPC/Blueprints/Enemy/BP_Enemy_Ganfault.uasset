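; Ganfault enemy NPC, a sword-wielding child of a parent enemy Blueprint.
; Its construction script runs the parent's, then creates a dynamic skin material, sets range, movement, combat and threat stats, and snaps the sword to its mesh socket.
; Attack events toggle EnableAttack on the Mixamo anim Blueprint, caching the instance on first attack.
; Killed increments the Ganfault kill counter in the game instance.
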(event `self.AttackAnim`
  ;[1 1 1] 攻击动画
  (if (== (`self.Anim`) null)
    (bind _asmixamo_anim_bp_gan_faul (cast `/Game/MixamoAnimPack/Mixamo_Ganfault/Anims/MixamoAnimBP_GanFaul` (`SkeletalMeshComponent.GetAnimInstance` (`self.Mesh`))))
    (set `self.Anim` _asmixamo_anim_bp_gan_faul))
  (if (not (`/Game/MixamoAnimPack/Mixamo_Ganfault/Anims/MixamoAnimBP_GanFaul.EnableAttack` (`self.Anim`)))
    (set `/Game/MixamoAnimPack/Mixamo_Ganfault/Anims/MixamoAnimBP_GanFaul.EnableAttack` true (`self.Anim`))))

(event `self.NotiAttackAnimCancel`
  ;[1 1 1] 取消攻击
  (bind _asmixamo_anim_bp_gan_faul (cast `/Game/MixamoAnimPack/Mixamo_Ganfault/Anims/MixamoAnimBP_GanFaul` (`SkeletalMeshComponent.GetAnimInstance` (`self.Mesh`))))
  (set `/Game/MixamoAnimPack/Mixamo_Ganfault/Anims/MixamoAnimBP_GanFaul.EnableAttack` false _asmixamo_anim_bp_gan_faul))

(event `self.Killed`
  (bind _assim_game_instance (cast `/Game/GameSave/SIM_GameInstance` (`GameplayStatics.GetGameInstance`)))
  (set `/Game/GameSave/SIM_GameInstance.KillNum_Ganfault` (+ (`/Game/GameSave/SIM_GameInstance.KillNum_Ganfault` _assim_game_instance) 1) _assim_game_instance))

(fn `UserConstructionScript`
  (bind __maxhealth (`self._MaxHealth`))
  (`parent.UserConstructionScript`)
  (bind _returnvalue (`PrimitiveComponent.CreateDynamicMaterialInstance` (`self.Mesh`) 1 "/Game/MixamoAnimPack/Mixamo_Ganfault/Materials/Ganfaul_Mat.Ganfaul_Mat"))
  (set `self.skin_MID` _returnvalue)
  (set `self.AttackRange` (`self._AttackRange`))
  (set `self.SenseRange` (`self._SenseRange`))
  (set `self.ThreatRange` (`self._ThreatRange`))
  (set `self.bCrossWall` (`self._bCrossWall`))
  (set `self.bLongDistance` (`self._bLongDistance`))
  (set `self.RunSpeed` (`self._RunSpeed`))
  (set `self.StopDistance` (`self._StopDistance`))
  (set `self.Damage` (`self._Damage`))
  (set `self.Name` (`self._Name`))
  (set `self.CurrentHealth` __maxhealth)
  (set `self.MaxHealth` __maxhealth)
  (set `self.PatrolThreatRemoveTime` (`self._PatrolThreatRemoveTime`))
  (set `self.AttackedThreatRemoveTime` (`self._AttackedThreatRemove`))
  (`SceneComponent.K2_AttachTo` (`self.Sword`) (`self.Mesh`) "Sword" "SnapToTargetIncludingScale" true)
  (set `self.Level` 5))