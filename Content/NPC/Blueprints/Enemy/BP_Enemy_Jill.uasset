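; BP_Enemy_Jill is the Jill enemy NPC, built on a parent enemy Blueprint.
; Its construction script runs the parent's, creates a dynamic skin material, assigns combat, sensing and movement stats, fills health, and sets pickups for a fixed level.
; Attack events toggle EnableAttack on the Mixamo AnimBP: AttackAnim caches the instance and turns it on, while NotiAttackAnimCancel turns it off.
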(event `self.AttackAnim`
  ;[1 1 1] Attack
  (if (== (`self.Anim`) null)
    (bind _asmixamo_anim_bp_jill (cast `/Game/MixamoAnimPack/Mixamo_Jill/Anims/MixamoAnimBP_Jill` (`SkeletalMeshComponent.GetAnimInstance` (`self.Mesh`))))
    (set `self.Anim` _asmixamo_anim_bp_jill))
  (if (not (`/Game/MixamoAnimPack/Mixamo_Jill/Anims/MixamoAnimBP_Jill.EnableAttack` (`self.Anim`)))
    (set `/Game/MixamoAnimPack/Mixamo_Jill/Anims/MixamoAnimBP_Jill.EnableAttack` true (`self.Anim`))))

(event `self.NotiAttackAnimCancel`
  ;[1 1 1] 停止攻击
  (bind _asmixamo_anim_bp_jill (cast `/Game/MixamoAnimPack/Mixamo_Jill/Anims/MixamoAnimBP_Jill` (`SkeletalMeshComponent.GetAnimInstance` (`self.Mesh`))))
  (set `/Game/MixamoAnimPack/Mixamo_Jill/Anims/MixamoAnimBP_Jill.EnableAttack` false _asmixamo_anim_bp_jill))

(fn `UserConstructionScript`
  (bind __maxhealth (`self._MaxHealth`))
  (`parent.UserConstructionScript`)
  (bind _returnvalue (`PrimitiveComponent.CreateDynamicMaterialInstance` (`self.Mesh`) 0 "/Game/MixamoAnimPack/Mixamo_Jill/Materials/Jill_Mat.Jill_Mat"))
  (set `self.skin_MID` _returnvalue)
  (set `self.AttackRange` (`self._AttackRange`))
  (set `self.SenseRange` (`self._SenseRange`))
  (set `self.ThreatRange` (`self._ThreatRange`))
  (set `self.bCrossWall` (`self._bCrossWall`))
  (set `self.bLongDistance` (`self._bLongDistance`))
  (set `self.RunSpeed` (`self._RunSpeed`))
  (set `self.StopDistance` (`self._StopDistance`))
  (set `self.Damage` (`self._Damage`))
  (set `self.Name` (`self._Name`))
  (set `self.CurrentHealth` __maxhealth)
  (set `self.MaxHealth` __maxhealth)
  (set `self.PatrolThreatRemoveTime` (`self._PatrolThreatRemoveTime`))
  (set `self.AttackedThreatRemoveTime` (`self._AttackedThreatRemove`))
  (bind _output_get (set `self.Level` 2))
  (`self.SetPickupsByLevel` _output_get))