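; Goblin enemy Blueprint that supplies attack animation control and per-type combat stats on top of a parent enemy class.
; AttackAnim sets EnableAttack on the Mixamo goblin AnimBP and briefly pulses the skinColor material parameter, while AttackAnimCancel clears the flag.
; The construction script runs the parent's, creates the dynamic skin material and assigns range, movement, damage, health, name and threat-timeout settings, with health starting at max.
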(event `self.AttackAnim`
  ;[1 1 1] Attack
  (if (== (`self.Anim`) null)
    (bind _asmixamo_anim_bp_goblin (cast `/Game/MixamoAnimPack/Mixamo_Goblin/Anims/MixamoAnimBP_Goblin` (`SkeletalMeshComponent.GetAnimInstance` (`self.Mesh`))))
    (set `self.Anim` _asmixamo_anim_bp_goblin))
  (if (not (`/Game/MixamoAnimPack/Mixamo_Goblin/Anims/MixamoAnimBP_Goblin.EnableAttack` (`self.Anim`)))
    (set `/Game/MixamoAnimPack/Mixamo_Goblin/Anims/MixamoAnimBP_Goblin.EnableAttack` true (`self.Anim`)))
  (`MaterialInstanceDynamic.SetScalarParameterValue` (`self.skin_MID`) "skinColor" 0.7)
  (`KismetSystemLibrary.Delay` 0.5)
  (`MaterialInstanceDynamic.SetScalarParameterValue` (`self.skin_MID`) "skinColor" 0.0))

(event `self.AttackAnimCancel`
  (bind _asmixamo_anim_bp_goblin (cast `/Game/MixamoAnimPack/Mixamo_Goblin/Anims/MixamoAnimBP_Goblin` (`SkeletalMeshComponent.GetAnimInstance` (`self.Mesh`))))
  (set `/Game/MixamoAnimPack/Mixamo_Goblin/Anims/MixamoAnimBP_Goblin.EnableAttack` false _asmixamo_anim_bp_goblin))

(fn `UserConstructionScript`
  (bind __maxhealth (`self._MaxHealth`))
  (`parent.UserConstructionScript`)
  (bind _returnvalue (`PrimitiveComponent.CreateDynamicMaterialInstance` (`self.Mesh`) 0 "/Game/MixamoAnimPack/Mixamo_Goblin/Materials/Goblin_mat.Goblin_mat"))
  (set `self.skin_MID` _returnvalue)
  (set `self.AttackRange` (`self._AttackRange`))
  (set `self.SenseRange` (`self._SenseRange`))
  (set `self.ThreatRange` (`self._ThreatRange`))
  (set `self.bCrossWall` (`self._bCrossWall`))
  (set `self.bLongDistance` (`self._bLongDistance`))
  (set `self.RunSpeed` (`self._RunSpeed`))
  (set `self.StopDistance` (`self._StopDistance`))
  (set `self.Damage` (`self._Damage`))
  (set `self.Name` (`self._Name`))
  (set `self.CurrentHealth` __maxhealth)
  (set `self.MaxHealth` __maxhealth)
  (set `self.PatrolThreatRemoveTime` (`self._PatrolThreatRemoveTime`))
  (set `self.AttackedThreatRemoveTime` (`self._AttackedThreatRemove`)))