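; Battery-named pickup actor that spins in place and hands its item info to a character on overlap.
; Tick yaws the mesh by RotateSpeed; trigger overlap with a BPI_Char implementer sets FromPlayer, sends PickUpItemMessage, then destroys the actor.
; The construction script calls its parent, then fills the info with a random count, the Pickups_Ammo class and the ammo HUD image, despite the Battery name.
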(event `self.ReceiveTick`
  (params (DeltaSeconds :type "Float (single-precision)"))
  ;[1 1 1] Auto Rotate
  (`SceneComponent.K2_AddLocalRotation` (`self.StaticMesh`) (`KismetMathLibrary.MakeRotator` 0.0 0.0 (* (`self.RotateSpeed`) DeltaSeconds)) false false))

(event `self.Trigger.OnComponentBeginOverlap`
  (params (OtherActor :type "Actor Object Reference") (OtherComp :type "PrimitiveComponent Object Reference") (OtherBodyIndex :type Integer) (bFromSweep :type Boolean) (SweepResult :type "HitResult Structure (by ref)"))
  ;[1 1 1] Pickup
  (if (`KismetSystemLibrary.DoesImplementInterface` OtherActor "/Game/FirstPersonBP/Interfaces/BPI_Char.BPI_Char_C")
    (set `self.bFromPlayer` true)
    (message `/Game/FirstPersonBP/Interfaces/BPI_Char.PickUpItem` OtherActor (make `/Game/Pickups/PickupInfo` (`self.PName`) (`self.PNum`) (`self.PClass`) (`self.PImage`)))
    (`self.K2_DestroyActor`)))

(fn `UserConstructionScript`
  (`parent.UserConstructionScript`)
  (bind _output_get (set `self.AmmoNum` (`KismetMathLibrary.RandomIntegerInRange` 2 15)))
  (set `self.PNum` _output_get)
  (set `self.PClass` "/Game/Pickups/Blueprints/Pickups_Ammo.Pickups_Ammo_C")
  (set `self.PName` (`self._PName`))
  (set `self.PImage` "/Game/UI/Items/HUD_ammo.HUD_ammo"))