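; BP_Key is a pickup key that spins in place and is collected when a character overlaps it.
; Tick rotates the static mesh around yaw at RotateSpeed, scaled by delta time.
; On trigger overlap, actors implementing BPI_Char receive GetKeyMessage with key info built from RoomId, then the key destroys itself.
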(event `self.ReceiveTick`
  (params (DeltaSeconds :type "Float (single-precision)"))
  ;[1 1 1] 旋转
  (`SceneComponent.K2_AddLocalRotation` (`self.StaticMesh`) (`KismetMathLibrary.MakeRotator` 0.0 0.0 (* (`self.RotateSpeed`) DeltaSeconds)) false false))

(event `self.Trigger.OnComponentBeginOverlap`
  (params (OtherActor :type "Actor Object Reference") (OtherComp :type "PrimitiveComponent Object Reference") (OtherBodyIndex :type Integer) (bFromSweep :type Boolean) (SweepResult :type "HitResult Structure (by ref)"))
  ;[1 1 1] 拾取
  (if (`KismetSystemLibrary.DoesImplementInterface` OtherActor "/Game/FirstPersonBP/Interfaces/BPI_Char.BPI_Char_C")
    (message `/Game/FirstPersonBP/Interfaces/BPI_Char.GetKey` OtherActor (make `/Game/Pickups/KeyInfo` (`self.RoomId`)))
    (`self.K2_DestroyActor`)))

(fn `UserConstructionScript`)