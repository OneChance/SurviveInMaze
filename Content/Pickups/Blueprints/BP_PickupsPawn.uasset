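; BP_PickupsPawn represents a pickup type, chosen by its PClass variable, with a matching billboard icon.
; The construction script compares PClass against the battery, ammo and key pickup classes and sets the Billboard sprite accordingly, leaving it unchanged for any other class.
; The event graph holds only disabled placeholder events, so this Blueprint's graphs contain no runtime spawning or collection logic.
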(event `self.ReceiveBeginPlay`)

(event `self.ReceiveActorBeginOverlap`
  (params (OtherActor :type "Actor Object Reference")))

(event `self.ReceiveTick`
  (params (DeltaSeconds :type "Float (single-precision)")))

(fn `UserConstructionScript`
  (if (== (`self.PClass`) "/Game/Pickups/Blueprints/Pickups_Battery.Pickups_Battery_C")
    (`BillboardComponent.SetSprite` (`self.Billboard`) "/Game/Pickups/Blueprints/battery_bb.battery_bb")
    (elif (== (`self.PClass`) "/Game/Pickups/Blueprints/Pickups_Ammo.Pickups_Ammo_C")
      (`BillboardComponent.SetSprite` (`self.Billboard`) "/Game/Pickups/Blueprints/ammo_bb.ammo_bb")
      (elif (== (`self.PClass`) "/Game/Pickups/Blueprints/BP_Key.BP_Key_C")
        (`BillboardComponent.SetSprite` (`self.Billboard`) "/Game/Pickups/Blueprints/key.key")))))